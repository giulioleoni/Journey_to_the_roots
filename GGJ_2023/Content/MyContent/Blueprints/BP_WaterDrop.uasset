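; BP_WaterDrop is a falling hazard actor that damages actors tagged Player and respawns at its start position.
; Each Tick sets the Sphere's relative location two units below the actor location, a fixed per-frame step without sweep or delta time.
; Overlapping a Player prints a collision message and applies damage.
; Any overlap, non-player hit, or Z below zero returns it to the location saved at BeginPlay.
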(event OnComponentBeginOverlap(Sphere)
  (params (OverlappedComponent :type Primitive%20Component%20Object%20Reference) (OtherActor :type Actor%20Object%20Reference) (OtherComp :type Primitive%20Component%20Object%20Reference) (OtherBodyIndex :type Integer) (bFromSweep :type Boolean) (SweepResult :type Hit%20Result%20Structure%20%28by%20ref%29))
  (if (Actor|ActorHasTag OtherActor "Player")
    (Development|PrintString "Collision" true true "(R=1.000000,G=0.027325,B=0.000000,A=1.000000)" 5.0)
    (Game|Damage|ApplyDamage OtherActor 1e+02 0 0))
  (Transformation|SetActorLocation (Variables|Default|GetStartingLocation) false false))

(event OnComponentHit(Sphere)
  (params (HitComponent :type Primitive%20Component%20Object%20Reference) (OtherActor :type Actor%20Object%20Reference) (OtherComp :type Primitive%20Component%20Object%20Reference) (NormalImpulse :type Vector :default "0, 0, 0") (Hit :type Hit%20Result%20Structure%20%28by%20ref%29))
  (if (not (Actor|ActorHasTag OtherActor "Player"))
    (Transformation|SetActorLocation (Variables|Default|GetStartingLocation) false false)))

(event EventBeginPlay
  (Variables|Default|SetStartingLocation (Transformation|GetActorLocation)))

(event EventTick
  (params (DeltaSeconds :type Float%20%28single-precision%29))
  (Transformation|SetRelativeLocation (Variables|Default|GetSphere) (+ (Transformation|GetActorLocation) "0,0.000000,-2.000000") false false)
  (if (< (.z (Transformation|GetActorLocation)) 0.0)
    (Transformation|SetActorLocation (Variables|Default|GetStartingLocation) false false)))

(fn ConstructionScript)